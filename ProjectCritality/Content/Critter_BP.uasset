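; Critter actor representing a player, with ID, nickname and transform initialised from a PlayerCrumb record.
; SetPosition places it immediately, while GoToPosition stores a converted target and sets yaw, both using BcPosToWorld scaled by 100.
; Tick refreshes the nickname text and, behind a position comparison, steps toward the target by Speed and delta time with sweep.
; Planar coordinates swap X and Y when read from or written to the actor location.
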(event `self.ReceiveTick`
  (params (DeltaSeconds :type "Float (single-precision)"))
  (bind _pendingpos (`self.pendingPos`))
  (`TextRenderComponent.K2_SetText` (`self.TextRender`) (`KismetTextLibrary.Conv_StringToText` (`self.nickname`)))
  (bind _pos (`self.getPos`))
  (if (not (`KismetMathLibrary.NotEqualExactly_Vector2DVector2D` _pos _pendingpos))
    (bind _pos_2 (`self.getPos`))
    (bind (_returnvalue_x _returnvalue_y) (`KismetMathLibrary.BreakVector2D` (+ _pos_2 (* (`KismetMathLibrary.Normal2D` (- _pendingpos _pos)) (* (`self.speed`) DeltaSeconds 100.0)))))
    (`self.K2_SetActorLocation` (`KismetMathLibrary.MakeVector` _returnvalue_y _returnvalue_x) true)))

(fn `getPos`
  (returns (pos :type "Vector2D Structure"))
  (bind (_returnvalue_x _returnvalue_y) (`KismetMathLibrary.BreakVector` (`self.K2_GetActorLocation`)))
  (return (`KismetMathLibrary.MakeVector2D` _returnvalue_y _returnvalue_x)))

(fn `goToPosition`
  (params (pos :type "Vector2D Structure") (rot :type "Float (double-precision)"))
  (bind _worldpos (`/Game/functions/BCPosConverter.bcPosToWorld` (`KismetMathLibrary.MakeVector2D` pos_X pos_Y)))
  (set `self.pendingPos` (* (`KismetMathLibrary.MakeVector2D` (`KismetMathLibrary.BreakVector2D` _worldpos) (`.Y` (`KismetMathLibrary.BreakVector2D` _worldpos))) 100.0))
  (`self.K2_SetActorRotation` (`KismetMathLibrary.MakeRotator` 0.0 0.0 rot)))

(fn `setPosition`
  (params (pos :type "Vector2D Structure") (rot :type "Float (double-precision)"))
  (bind _worldpos (`/Game/functions/BCPosConverter.bcPosToWorld` (`KismetMathLibrary.MakeVector2D` pos_X pos_Y)))
  (`self.K2_SetActorLocation` (* (`KismetMathLibrary.MakeVector` (`.Y` (`KismetMathLibrary.BreakVector2D` _worldpos)) (`KismetMathLibrary.BreakVector2D` _worldpos)) 100.0) true)
  (`self.K2_SetActorRotation` (`KismetMathLibrary.MakeRotator` 0.0 0.0 rot)))

(fn `setupProperties`
  (params (playerCrumb :type "/Game/crumbs/playerCrumb Structure"))
  (bind (_i _n _x _y _r) (break `/Game/crumbs/playerCrumb` playerCrumb))
  (set `self.id` _i)
  (set `self.nickname` _n)
  (`self.setPosition` (`KismetMathLibrary.MakeVector2D` _x _y) _r))

(fn `UserConstructionScript`)