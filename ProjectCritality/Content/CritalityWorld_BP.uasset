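; CritalityWorld actor is the multiplayer client that connects to the game server over Socket.IO and mirrors a room's players.
; On BeginPlay it connects, binds the event names and emits a login with username and ticket.
; The login reply triggers a join to the hardcoded "tavern", whose response spawns and sets up a Room_BP.
; Short-code events then forward player adds, removals, teleport moves and chat balloons to that room, with debug printing throughout.
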(event `self.ReceiveBeginPlay`
  (`SocketIOClientComponent.Connect` (`self.SocketIOClient`) (`self.serverURL`) null null)
  (`self.socketHandler`)
  (`self.login` (`self.username`)))

(event `self.SocketIOClient.OnConnected`
  (params (SessionId :type String) (bIsReconnection :type Boolean))
  (`KismetSystemLibrary.PrintString` "Connected" true true (struct :`G` 0.66 :`B` 1.0 :`A` 1.0) 99.0))

(event `self.SocketIOClient.OnDisconnected`
  (params (Reason :type "ESIOConnectionCloseReason Enum" :default "CLOSE_REASON_NORMAL"))
  (`KismetSystemLibrary.PrintString` "DISCONNECTED" true true (struct :`G` 0.66 :`B` 1.0 :`A` 1.0) 98.0))

(event `self.SocketIOClient.OnFail`
  (`KismetSystemLibrary.PrintString` "Connection Failed" true true (struct :`G` 0.66 :`B` 1.0 :`A` 1.0) 98.0 :!label _label))

(event `self.SocketIOClient.OnConnectionProblems`
  (params (Attempts :type Integer) (NextAttemptInMs :type Integer) (TimeSinceConnected :type "Float (single-precision)"))
  (goto _label))

(event `self.SocketIOClient.OnEvent`
  (params (Event :type String) (MessageJson :type "SIOJsonValue Object Reference"))
  (bind _logincrumb (make `/Game/crumbs/loginCrumb` "" "" (`|MakeArray` "")))
  (switch `string` Event
    (:`login`
      ;[1 1 1] Login
      (`self.printSocketInfo` Event MessageJson)
      (bind _returnvalue (`SIOJsonObject.ConstructJsonObject`))
      (`SIOJsonObject.SetStringField` _returnvalue "roomId" "tavern")
      (`SocketIOClientComponent.Emit` (`self.SocketIOClient`) "joinRoom" (`SIOJsonValue.ConstructJsonValueObject` _returnvalue) "/")
      (`SIOJLibrary.JsonObjectToStruct` _returnvalue _logincrumb)
      (set `self.playerID` (`.playerId_6_CD14188A4D2664B163666CA644DDF5A5` (break `/Game/crumbs/loginCrumb` _logincrumb))))
    (:`joinRoom`
      ;[1 1 1] joinRoom
      (`self.printSocketInfo` Event MessageJson)
      (bind _room (`self.createRoom` MessageJson))
      (bind _player (`/Game/Room_BP.getPlayer` _room ""))
      (set `self.playerCritter` _player))
    (:`A`
      ;[1 1 1] A
      (`self.printSocketInfo` Event MessageJson)
      (`/Game/Room_BP.addPlayerJSON` (`self.room`) MessageJson))
    (:`M`
      ;[1 1 1] M
      (`self.printSocketInfo` Event MessageJson)
      (`/Game/Room_BP.addBalloon` (`self.room`) MessageJson))
    (:`P`
      ;[1 1 1] P
      (`self.printSocketInfo` Event MessageJson)
      (`/Game/Room_BP.movePlayer` (`self.room`) MessageJson true))
    (:`R`
      ;[1 1 1] R
      (`self.printSocketInfo` Event MessageJson)
      (`/Game/Room_BP.removePlayer` (`self.room`) MessageJson))))

(fn `createRoom`
  (params (roomCrumb :type "SIOJsonValue Object Reference"))
  (returns (room :type "/Game/Room_BP Object Reference"))
  (locals (newRoomInfo :type "/Game/crumbs/roomCrumb Structure"))
  (bind _output_get (set `local.newRoomInfo` (make `/Game/crumbs/roomCrumb` "" "" (`|MakeArray` (struct) :!type "/Game/crumbs/playerCrumb Structure"))))
  (bind _returnvalue (`SIOJLibrary.JsonObjectToStruct` (`SIOJLibrary.Conv_JsonValueToJsonObject` roomCrumb) _output_get))
  (if _returnvalue
    (`self.printSocketInfo` "createRoom" roomCrumb)
    (bind _returnvalue_2 (`|SpawnActorFromClass` "/Game/Room_BP.Room_BP_C" (`KismetMathLibrary.MakeTransform` (0.0 0.0 -10.0) (struct) (1.0 1.0 0.2)) "Undefined" "OverrideRootScale" null null))
    (bind _output_get_2 (set `self.room` _returnvalue_2))
    (`/Game/Room_BP.setupProperties` _output_get_2 (`local.newRoomInfo`))
    (return _output_get_2)
    (else
      (`KismetSystemLibrary.PrintString` "failed to create room"))))

(fn `login`
  (params (username :type String))
  (bind _returnvalue (`SIOJsonObject.ConstructJsonObject`))
  (`SIOJsonObject.SetStringField` _returnvalue "username" username)
  (`SIOJsonObject.SetStringField` _returnvalue "ticket" (`self.ticket`))
  (`SocketIOClientComponent.Emit` (`self.SocketIOClient`) "login" (`SIOJsonValue.ConstructJsonValueObject` _returnvalue) "/"))

(fn `printSocketInfo`
  (params (Event :type String) (messageJSON :type "SIOJsonValue Object Reference"))
  (`KismetSystemLibrary.PrintString` (`KismetStringLibrary.Concat_StrStr` Event " " (`SIOJsonValue.EncodeJson` messageJSON)) true true (struct :`G` 0.66 :`B` 1.0 :`A` 1.0) 99.0))

(fn `socketHandler`
  (for _array_element (`KismetStringLibrary.ParseIntoArray` "login,joinRoom,A,R,P,M" ",")
    (`SocketIOClientComponent.BindEvent` (`self.SocketIOClient`) _array_element "/")))

(fn `UserConstructionScript`)