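; Room actor that represents a multiplayer room and manages the BP_Critter characters standing in for its players.
; SetupProperties scales and positions the floor cube from a RoomCrumb, calls critter navmesh setup and spawns the initial players.
; JSON crumbs are converted to structs to add, remove, walk or teleport critters, looked up through parallel ID and player arrays.
; AddBalloon only parses its message and displays nothing yet.
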(fn `addBalloon`
  (params (messageCrumb :type "SIOJsonValue Object Reference"))
  (locals (messageInfo :type "/Game/Blueprints/Structs/messageCrumb Structure"))
  (bind _output_get (set `local.messageInfo` (make `/Game/Blueprints/Structs/messageCrumb` "")))
  (`SIOJLibrary.JsonObjectToStruct` (`SIOJLibrary.Conv_JsonValueToJsonObject` messageCrumb) _output_get))

(fn `addPlayer`
  (params (playerCrumb :type "/Game/Blueprints/Structs/playerCrumb Structure"))
  (locals (newplayer :type "/Game/Blueprints/Game/BP_Critter Object Reference"))
  (bind ((`i_12_94C25E4E4805FE429981E493A3AD71F4` _i) (`n_13_80C65B7E44ACFC7AA375259E1A7D2C48` _n)) (break `/Game/Blueprints/Structs/playerCrumb` playerCrumb))
  (`KismetSystemLibrary.PrintString` (`KismetStringLibrary.Concat_StrStr` _i " " _n) true true (struct :`G` 0.66 :`B` 1.0 :`A` 1.0) 99.0)
  (`KismetArrayLibrary.Array_Add` (`self.idList`) _i)
  (bind _returnvalue (`|SpawnActorFromClass` "/Game/Blueprints/Game/BP_Critter.BP_Critter_C" (`KismetMathLibrary.MakeTransform` (0.0 0.0 10.0)) "Undefined" "OverrideRootScale" null null))
  (bind _output_get (set `local.newplayer` _returnvalue))
  (`/Game/Blueprints/Game/BP_Critter.setupProperties` _output_get playerCrumb self)
  (`KismetArrayLibrary.Array_Add` (`self.playerlist`) (`local.newplayer`)))

(fn `addPlayerJSON`
  (params (playerCrumb :type "SIOJsonValue Object Reference"))
  (locals (playerInfo :type "/Game/Blueprints/Structs/playerCrumb Structure"))
  (bind _output_get (set `local.playerInfo` (make `/Game/Blueprints/Structs/playerCrumb` "")))
  (`SIOJLibrary.JsonObjectToStruct` (`SIOJLibrary.Conv_JsonValueToJsonObject` playerCrumb) _output_get)
  (`self.addPlayer` (`local.playerInfo`)))

(fn `getPlayer`
  (params (playerId :type String))
  (returns (player :type "/Game/Blueprints/Game/BP_Critter Object Reference") (index :type Integer))
  (bind _returnvalue (`KismetArrayLibrary.Array_Find` (`self.idList`) playerId))
  (return (`|GetArrayItem` (`self.playerlist`) _returnvalue) _returnvalue))

(fn `movePlayer`
  (params (moveCrumb :type "SIOJsonValue Object Reference") (teleport :type Boolean))
  (locals (moveInfo :type "/Game/Blueprints/Structs/moveCrumb Structure"))
  (bind (_i _x _y _r) (break `/Game/Blueprints/Structs/moveCrumb` (`local.moveInfo`)))
  (bind _output_get (set `local.moveInfo` (make `/Game/Blueprints/Structs/moveCrumb`)))
  (`SIOJLibrary.JsonObjectToStruct` (`SIOJLibrary.Conv_JsonValueToJsonObject` moveCrumb) _output_get)
  (bind _player (`self.getPlayer` _i))
  (if teleport
    (`/Game/Blueprints/Game/BP_Critter.setPosition` _player (`KismetMathLibrary.MakeVector2D` _x _y) _r self)
    (else
      (`/Game/Blueprints/Game/BP_Critter.goToPosition` _player (`KismetMathLibrary.MakeVector2D` _x _y) _r self))))

(fn `removePlayer`
  (params (playerCrumb :type "SIOJsonValue Object Reference"))
  (locals (playerInfo :type "/Game/Blueprints/Structs/playerCrumb Structure"))
  (bind _output_get (set `local.playerInfo` (make `/Game/Blueprints/Structs/playerCrumb` "")))
  (`SIOJLibrary.JsonObjectToStruct` (`SIOJLibrary.Conv_JsonValueToJsonObject` playerCrumb) _output_get)
  (bind (_player _index) (`self.getPlayer` (`.i_12_94C25E4E4805FE429981E493A3AD71F4` (break `/Game/Blueprints/Structs/playerCrumb` (`local.playerInfo`)))))
  (`KismetArrayLibrary.Array_Remove` (`self.playerlist`) _index)
  (`KismetArrayLibrary.Array_Remove` (`self.idList`) _index)
  (`self.K2_DestroyActor` _player))

(fn `setupProperties`
  (params (roomCrumb :type "/Game/Blueprints/Structs/roomCrumb Structure"))
  (bind (_roomid _name _width _height _playerlist) (break `/Game/Blueprints/Structs/roomCrumb` roomCrumb))
  (bind _cube (`self.Cube`))
  (bind (_returnvalue_x _returnvalue_y _returnvalue_z) (`KismetMathLibrary.BreakVector` (`SceneComponent.K2_GetComponentScale` (`self.Cube`))))
  (bind (_returnvalue_x_2 _returnvalue_y_2 _returnvalue_z_2) (`KismetMathLibrary.BreakVector` (`SceneComponent.K2_GetComponentScale` _cube)))
  (set `self.roomId` _roomid)
  (set `self.name` _name)
  (bind _worldpos (`/Game/Blueprints/Game/BCPosConverter.bcPosToWorld` (`KismetMathLibrary.MakeVector2D` _width _height)))
  (bind _output_get (set `self.width` (`.Y` (`KismetMathLibrary.BreakVector2D` _worldpos))))
  (bind _output_get_2 (set `self.height` (`KismetMathLibrary.BreakVector2D` _worldpos)))
  (`SceneComponent.SetWorldScale3D` _cube (`KismetMathLibrary.MakeVector` _output_get_2 _output_get _returnvalue_z_2))
  (`self.K2_SetActorLocation` (`KismetMathLibrary.MakeVector` (* _returnvalue_x 50.0) (* _returnvalue_y 50.0) (* _returnvalue_z -50.0)))
  (`self.SetupCritterMoveAINavMesh` (`KismetMathLibrary.MakeTransform` (`self.K2_GetActorLocation`) (struct) (`SceneComponent.K2_GetComponentScale` (`self.Cube`))))
  (for _array_element _playerlist
    (`self.addPlayer` _array_element)))

(fn `UserConstructionScript`)