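; BP_PlayerCritter is a VR player actor that enables input and sets a floor tracking origin on BeginPlay.
; Left and right grab inputs drive left mouse clicks through per-hand widget interaction components for pointing at UI.
; Each component's debug laser appears only while it hovers a valid widget.
; The right grab release calls ReleaseKey, while the left calls ReleasePointerKey.
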(event `self.ReceiveBeginPlay`
  ;[1 1 1] Setup
  (`self.EnableInput` (`GameplayStatics.GetPlayerController` 0))
  (`HeadMountedDisplayFunctionLibrary.SetTrackingOrigin` "Floor"))

(event `InputAction|VR_Grab_L`
  (params (Key :type "Key Structure"))
  (bind _wi_left (`self.WI_Left`))
  ;[1 1 1] Pointer Click
  (:`Pressed`
    (`WidgetInteractionComponent.PressPointerKey` _wi_left "LeftMouseButton"))
  (:`Released`
    (`WidgetInteractionComponent.ReleasePointerKey` _wi_left "LeftMouseButton")))

(event `self.WI_Left.OnHoveredWidgetChanged`
  (params (WidgetComponent :type "WidgetComponent Object Reference") (PreviousWidgetComponent :type "WidgetComponent Object Reference"))
  ;[1 1 1] Auto Lasor
  (set `WidgetInteractionComponent.bShowDebug` (`KismetSystemLibrary.IsValid` WidgetComponent) (`self.WI_Left`)))

(event `InputAction|VR_Grab_R`
  (params (Key :type "Key Structure"))
  (bind _wi_right (`self.WI_Right`))
  ;[1 1 1] Pointer Click
  (:`Pressed`
    (`WidgetInteractionComponent.PressPointerKey` _wi_right "LeftMouseButton"))
  (:`Released`
    (`WidgetInteractionComponent.ReleaseKey` _wi_right "LeftMouseButton")))

(event `self.WI_Right.OnHoveredWidgetChanged`
  (params (WidgetComponent :type "WidgetComponent Object Reference") (PreviousWidgetComponent :type "WidgetComponent Object Reference"))
  ;[1 1 1] Auto Lasor
  (set `WidgetInteractionComponent.bShowDebug` (`KismetSystemLibrary.IsValid` WidgetComponent) (`self.WI_Right`)))

(fn `UserConstructionScript`)