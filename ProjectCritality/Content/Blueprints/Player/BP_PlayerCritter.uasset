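; Player critter with VR support: on a head-mounted display it hides its cube and spawns left and right motion controllers.
; Grab inputs drive each controller's pointer; teleport inputs aim, and release triggers a camera fade.
; Teleporting sends the destination as a click to CritalityInstance instead of moving the actor directly.
; After setup or look-at, the VR camera root's world rotation is zeroed and its relative rotation is copied to both controllers.
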(event `self.ReceiveBeginPlay`
  (bind _returnvalue (`self.GetTransform`))
  ;[1 1 1] Setup
  (`self.EnableInput` (`GameplayStatics.GetPlayerController` 0))
  (if (`HeadMountedDisplayFunctionLibrary.IsHeadMountedDisplayEnabled`)
    (`HeadMountedDisplayFunctionLibrary.SetTrackingOrigin` "Floor")
    (`SceneComponent.SetHiddenInGame` (`self.Cube`) true false)
    ;[1 1 1] Setup Motion Controllers
    ;;[1 1 1] Left
    (bind _returnvalue_2 (`|SpawnActorFromClass` "/Game/Blueprints/Player/BP_MotionController.BP_MotionController_C" _returnvalue "AlwaysSpawn" "OverrideRootScale" self null))
    (bind _output_get (set `self.MC_Left` _returnvalue_2))
    (`/Game/Blueprints/Player/BP_MotionController.SetHand` _output_get "Left")
    ;;[1 1 1] Right
    (bind _returnvalue_3 (`|SpawnActorFromClass` "/Game/Blueprints/Player/BP_MotionController.BP_MotionController_C" _returnvalue "AlwaysSpawn" "OverrideRootScale" self null))
    (bind _output_get_2 (set `self.MC_Right` _returnvalue_3))
    (`/Game/Blueprints/Player/BP_MotionController.SetHand` _output_get_2 "Right")))

(event `InputAction|VR_Teleport_L`
  (params (Key :type "Key Structure"))
  (bind _mc_left (`self.MC_Left`))
  ;[1 1 1] TeleportActivation
  (:`Pressed`
    (`/Game/Blueprints/Player/BP_MotionController.ActivateTeleporter` _mc_left))
  (:`Released`
    (if (`/Game/Blueprints/Player/BP_MotionController.shouldTrace` _mc_left)
      (set `self.teleportController` _mc_left)
      (`self.ExecuteTeleport`)
      (`/Game/Blueprints/Player/BP_MotionController.DisableTeleporter` _mc_left))))

(event `InputAction|VR_Grab_L`
  (params (Key :type "Key Structure"))
  (bind _mc_left (`self.MC_Left`))
  ;[1 1 1] Pointer Click
  (:`Pressed`
    (`/Game/Blueprints/Player/BP_MotionController.ClickPointer` _mc_left))
  (:`Released`
    (`/Game/Blueprints/Player/BP_MotionController.ReleasePointer` _mc_left)))

(event `InputAction|VR_Teleport_R`
  (params (Key :type "Key Structure"))
  (bind _mc_right (`self.MC_Right`))
  ;[1 1 1] TeleportActivation
  (:`Pressed`
    (`/Game/Blueprints/Player/BP_MotionController.ActivateTeleporter` _mc_right))
  (:`Released`
    (if (`/Game/Blueprints/Player/BP_MotionController.shouldTrace` _mc_right)
      (set `self.teleportController` _mc_right)
      (`self.ExecuteTeleport`)
      (`/Game/Blueprints/Player/BP_MotionController.DisableTeleporter` _mc_right))))

(event `InputAction|VR_Grab_R`
  (params (Key :type "Key Structure"))
  (bind _mc_right (`self.MC_Right`))
  ;[1 1 1] Pointer Click
  (:`Pressed`
    (`/Game/Blueprints/Player/BP_MotionController.ClickPointer` _mc_right))
  (:`Released`
    (`/Game/Blueprints/Player/BP_MotionController.ReleasePointer` _mc_right)))

(event `ExecuteTeleport`
  (bind _fadeduration (`self.fadeDuration`))
  ;[1 1 1] Execute Teleport
  (if (`/Game/Blueprints/Player/BP_MotionController.traceSuccess` (`self.teleportController`))
    (`PlayerCameraManager.StartCameraFade` :`self` (`GameplayStatics.GetPlayerCameraManager` 0) :`ToAlpha` 1.0 :`Duration` _fadeduration :`bHoldWhenFinished` true)
    (`KismetSystemLibrary.Delay` _fadeduration)
    (bind _ascritality_instance (cast `/Game/Blueprints/CritalityInstance` (`GameplayStatics.GetGameInstance`)))
    (`/Game/Blueprints/CritalityInstance.SendClick` _ascritality_instance (`/Game/Blueprints/Player/BP_MotionController.teleportDestination` (`self.teleportController`)))
    (`PlayerCameraManager.StartCameraFade` :`self` (`GameplayStatics.GetPlayerCameraManager` 0) :`FromAlpha` 1.0 :`Duration` (`self.fadeDuration`) :`bHoldWhenFinished` true)
    (set `self.teleportController` null)))

(event `self.setupProperties`
  (params (playerCrumb :type "/Game/Blueprints/Structs/playerCrumb Structure"))
  ;[1 1 1] VR Rotation
  (`parent.setupProperties` playerCrumb)
  (if (`HeadMountedDisplayFunctionLibrary.IsHeadMountedDisplayEnabled`) :!label _label
    (`self.updateVRRotation`)))

(event `self.lookAtPos`
  (params (Target :type "Vector Structure (by ref)"))
  ;[1 1 1] VR Rotation
  (`parent.lookAtPos` Target)
  (goto _label))

(fn `updateVRRotation`
  (bind _relativerotation (`SceneComponent.RelativeRotation` (`self.VRCameraRoot`)))
  (`SceneComponent.K2_SetWorldRotation` :`self` (`self.VRCameraRoot`))
  (`self.K2_SetActorRotation` (`self.MC_Left`) _relativerotation false)
  (`self.K2_SetActorRotation` (`self.MC_Right`) _relativerotation false))

(fn `UserConstructionScript`)