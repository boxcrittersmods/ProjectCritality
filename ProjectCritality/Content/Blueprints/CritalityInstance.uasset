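; Game instance that manages menu flow and the Socket.IO server connection.
; It opens MainMenu on init and lazily creates cached menu and loading screen widgets.
; ConnectToServer shows the loading screen and builds a socket that opens GameWorld on success; failure calls DisplayErrorMessage, an empty stub.
; Login emits the username with a placeholder player ID, the Ticket input goes unused, and Shutdown emits a disconnect.
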(event `self.ReceiveInit`
  ;[1 1 1] Start Game
  (`GameplayStatics.OpenLevel` "MainMenu"))

(event `ShowMainMenu`
  (bind _returnvalue (`GameplayStatics.GetPlayerController` 0))
  ;[1 1 1] Show Main Menu
  (`/Engine/EditorBlueprintResources/StandardMacros.IsValid` (`self.MainMenu_WB`)
    (:`Is Valid`
      _)
    (:`Is Not Valid`
      (bind _returnvalue_2 (`|CreateWidget` "/Game/UI/MainMenu/MainMenu.MainMenu_C" _returnvalue))
      (bind _output_get (set `self.MainMenu_WB` _returnvalue_2))))
  (`UserWidget.AddToViewport` _output_get 0)
  (set `PlayerController.bShowMouseCursor` true _returnvalue))

(event `ShowLoadingScreen`
  ;[1 1 1] Show Loading Screen
  (`/Engine/EditorBlueprintResources/StandardMacros.IsValid` (`self.loadingScreen_WB`)
    (:`Is Valid`
      _)
    (:`Is Not Valid`
      (bind _returnvalue (`|CreateWidget` "/Game/UI/MainMenu/LoadingScreen.LoadingScreen_C" (`GameplayStatics.GetPlayerController` 0)))
      (bind _output_get (set `self.loadingScreen_WB` _returnvalue))))
  (`UserWidget.AddToViewport` _output_get 0))

(event `ConnectToServer`
  (params (serverURL :type String) (username :type String) (ticket :type String))
  (bind _socket (`self.socket`))
  ;[1 1 1] Connect to Server
  (bind _output_get (set `self.serverURL` serverURL))
  (set `self.username` username)
  (`self.ShowLoadingScreen`)
  (bind _returnvalue (`SocketIOFunctionLibrary.ConstructSocketIOComponent`))
  (bind _output_get_2 (set `self.socket` _returnvalue))
  (`SocketIOClientComponent.Connect` _output_get_2 _output_get null null)
  (add `SocketIOClientComponent.OnConnected` _socket (delegate `SIO_Connected`))
  (add `SocketIOClientComponent.OnFail` _socket (delegate `SIO_Fail`)))

(event `SIO_Connected`
  (params (SessionId :type String) (bIsReconnection :type Boolean))
  ;[1 1 1] Connect to Server
  (`GameplayStatics.OpenLevel` "GameWorld"))

(event `SIO_Fail`
  ;[1 1 1] Connect to Server
  (`self.DisplayErrorMessage` "Failed to connect to server"))

(event `Login`
  ;[1 1 1] Login
  (bind _returnvalue (`SIOJsonObject.ConstructJsonObject`))
  (`SIOJsonObject.SetStringField` _returnvalue "playerId" "what would i put here?")
  (`SIOJsonObject.SetStringField` _returnvalue "nickname" (`self.username`))
  (`SocketIOClientComponent.Emit` (`self.socket`) "login" (`SIOJsonValue.ConstructJsonValueObject` _returnvalue) "/"))

(event `self.ReceiveShutdown`
  ;[1 1 1] Disconnect
  (`SocketIOClientComponent.Emit` (`self.socket`) "disconnect" (`SIOJsonValue.ConstructJsonValueString` "client closed") "/"))