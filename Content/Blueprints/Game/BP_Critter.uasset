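; BP_Critter is a player's critter avatar, initialized from a PlayerCrumb with ID, nickname, critter ID and position.
; GoToPosition converts Box Critters coordinates to Unreal space and moves a spawned BP_Pointer there as the target.
; Each Tick steps toward that pointer at constant speed while facing it, snapping on arrival.
; Tick also refreshes the nickname text and orients it to the camera view target's rotation, turned around.
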(event `self.ReceiveTick`
  (params (DeltaSeconds :type "Float (single-precision)"))
  (`self.updatePos` DeltaSeconds)
  (`self.updateNickname`)
  (if (`self.moving`)
    (`self.lookAtPos` (`self.K2_GetActorLocation` (`self.pendingPosPtr`)))))

(fn `getPos`
  (returns (pos :type "Vector2D Structure"))
  (bind (_returnvalue_x _returnvalue_y) (`KismetMathLibrary.BreakVector` (`self.K2_GetActorLocation`)))
  (return (`KismetMathLibrary.MakeVector2D` _returnvalue_x _returnvalue_y)))

(fn `goToPosition`
  (params (pos :type "Vector2D Structure"))
  (bind _returnvalue (`PosCoversion.BoxCrittersToUnreal` pos))
  (`self.lookAtPos` _returnvalue)
  (`self.K2_SetActorLocation` (`self.pendingPosPtr`) _returnvalue false false)
  (set `self.moving` true))

(fn `lookAtPos`
  (params (Target :type "Vector Structure (by ref)"))
  (`self.K2_SetActorRotation` (`KismetMathLibrary.FindLookAtRotation` (`self.K2_GetActorLocation`) Target)))

(fn `setPosition`
  (params (pos :type "Vector2D Structure"))
  (bind _returnvalue (`PosCoversion.BoxCrittersToUnreal` pos))
  (`self.K2_SetActorLocation` _returnvalue false true))

(fn `setupProperties`
  (params (playerCrumb :type "PlayerCrumb Structure"))
  (bind (_i _n _c _x _y) (break `PlayerCrumb` playerCrumb))
  (set `self.id` _i)
  (set `self.nickname` _n)
  (set `self.critterId` _c)
  (`self.setPosition` (`KismetMathLibrary.MakeVector2D` _x _y))
  (bind _returnvalue (`|SpawnActorFromClass` "/Game/Blueprints/BP_Pointer.BP_Pointer_C" (`KismetMathLibrary.MakeTransform` (0.0 0.0 0.0)) "Undefined" "OverrideRootScale" self null))
  (set `self.pendingPosPtr` _returnvalue))

(fn `updateNickname`
  (bind _textrender (`self.TextRender`))
  ;[1 1 1] Update Nickname
  (`TextRenderComponent.K2_SetText` (`self.TextRender`) (`KismetTextLibrary.Conv_StringToText` (`self.nickname`)))
  ;[1 1 1] Look At Camers
  (`SceneComponent.K2_SetWorldRotation` _textrender (.rotation (`self.GetTransform` (`Controller.GetViewTarget` (`GameplayStatics.GetPlayerController` 0)))) false false)
  (`SceneComponent.K2_AddLocalRotation` _textrender (struct :`Yaw` -180.0) false false))

(fn `updatePos`
  (params (delta :type "Float (double-precision)"))
  (locals (distanceVector :type "Vector Structure" :default (0.0 0.0 0.0)) (magnitude :type "Float (double-precision)" :default 0.0) (maxDistance :type "Float (double-precision)" :default 0.0))
  (if (`self.moving`)
    ;[1 1 1] Calculate Max Distance
    (set `local.maxDistance` (* delta (`self.speed`) 100.0))
    ;[1 1 1] DistanceVector
    (bind _output_get (set `local.distanceVector` (- (`self.K2_GetActorLocation` (`self.pendingPosPtr`)) (`self.K2_GetActorLocation`))))
    ;[1 1 1] Magnitude
    (bind _output_get_2 (set `local.magnitude` (`KismetMathLibrary.VSize` _output_get)))
    ;[1 1 1] magnitude<=speed || magnitude==0
    (if (or (<= _output_get_2 (`local.maxDistance`)) (== _output_get_2 0.0))
      ;[1 1 1] Arrive
      (`self.K2_SetActorLocation` (`self.K2_GetActorLocation` (`self.pendingPosPtr`)))
      (set `self.moving` false)
      (else
        ;[1 1 1] Move some more
        (`self.K2_SetActorLocation` (+ (`self.K2_GetActorLocation`) (* (/ (`local.distanceVector`) (`local.magnitude`)) (`local.maxDistance`))))))))

(fn `UserConstructionScript`)