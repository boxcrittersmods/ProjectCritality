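; BP_Room represents a multiplayer room, tracking its critters and applying join, leave and movement data received as JSON.
; SetupProperties parses the room crumb and adds each player; other functions parse their own crumbs and find critters through the ID-keyed Playerlist.
; AddPlayer reuses the local pawn when the username matches the game instance's, otherwise spawns a BP_Critter.
; MovePlayer either teleports or walks critters, while AddBalloon only parses its message so far.
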(fn `addBalloon`
  (params (messageCrumb :type "SIOJsonValue Object Reference"))
  (locals (messageInfo :type "/Game/Blueprints/Structs/BP_messageCrumb Structure"))
  (bind _output_get (set `local.messageInfo` (make `/Game/Blueprints/Structs/BP_messageCrumb` "")))
  (`SIOJLibrary.JsonObjectToStruct` (`SIOJLibrary.Conv_JsonValueToJsonObject` messageCrumb) _output_get))

(fn `addPlayer`
  (params (playerCrumb :type "PlayerCrumb Structure"))
  (locals (newPlayer :type "/Game/Blueprints/Game/BP_Critter Object Reference"))
  (bind (_i _n _c) (break `PlayerCrumb` playerCrumb))
  ;[1 1 1] Check for existing critter
  (bind _ascritality_instance (cast `/Game/Blueprints/CritalityInstance` (`GameplayStatics.GetGameInstance`)))
  (if (`KismetStringLibrary.EqualEqual_StrStr` (`/Game/Blueprints/CritalityInstance.username` _ascritality_instance) (`.n` (break `PlayerCrumb` playerCrumb)))
    ;[1 1 1] Check for existing player
    (bind _asbp_critter (cast `/Game/Blueprints/Game/BP_Critter` (`GameplayStatics.GetPlayerPawn` 0)))
    (set `local.newPlayer` _asbp_critter)
    (else
      ;[1 1 1] Create New CRitter
      (bind _returnvalue (`|SpawnActorFromClass` "/Game/Blueprints/Game/BP_Critter.BP_Critter_C" (`KismetMathLibrary.MakeTransform` (0.0 0.0 0.0)) "AlwaysSpawn" "OverrideRootScale" null null))
      (set `local.newPlayer` _returnvalue)))
  ;[1 1 1] Setup Player
  (`/Game/Blueprints/Game/BP_Critter.setupProperties` _returnvalue playerCrumb)
  (`/Game/Blueprints/Game/BP_Critter.setupProperties` (`local.newPlayer`) playerCrumb)
  (`BlueprintMapLibrary.Map_Add` (`self.playerlist`) _i (`local.newPlayer`))
  ;[1 1 1] Print Player Details
  (`KismetSystemLibrary.PrintString` (`KismetStringLibrary.Concat_StrStr` _i " " _n " " _c) true true (struct :`G` 0.66 :`B` 1.0 :`A` 1.0) 99.0))

(fn `addPlayerJSON`
  (params (playerCrumb :type "SIOJsonValue Object Reference"))
  (locals (newPlayer :type "PlayerCrumb Structure"))
  (bind _output_get (set `local.newPlayer` (make `PlayerCrumb` "")))
  (`SIOJLibrary.JsonObjectToStruct` (`SIOJLibrary.Conv_JsonValueToJsonObject` playerCrumb) _output_get)
  (`self.addPlayer` (`local.newPlayer`)))

(fn `movePlayer`
  (params (moveCrumb :type "SIOJsonValue Object Reference") (teleport :type Boolean))
  (locals (moveInfo :type "/Game/Blueprints/Structs/BP_moveCrumb Structure") (playerToMove :type "/Game/Blueprints/Game/BP_Critter Object Reference"))
  (bind (_i _x _y) (break `/Game/Blueprints/Structs/BP_moveCrumb` (`local.moveInfo`)))
  (bind _output_get (set `local.moveInfo` (make `/Game/Blueprints/Structs/BP_moveCrumb`)))
  (`SIOJLibrary.JsonObjectToStruct` (`SIOJLibrary.Conv_JsonValueToJsonObject` moveCrumb) _output_get)
  (set `local.playerToMove` (`BlueprintMapLibrary.Map_Find` (`self.playerlist`) _i))
  (if teleport
    (`/Game/Blueprints/Game/BP_Critter.setPosition` (`local.playerToMove`) (`KismetMathLibrary.MakeVector2D` _x _y))
    (else
      (`/Game/Blueprints/Game/BP_Critter.goToPosition` (`local.playerToMove`) (`KismetMathLibrary.MakeVector2D` _x _y)))))

(fn `removePlayer`
  (params (playerCrumb :type "SIOJsonValue Object Reference"))
  (locals (playerCrumbToDelete :type "/Game/Blueprints/Structs/BP_playerCrumb Structure") (playerToDelete :type "/Game/Blueprints/Game/BP_Critter Object Reference"))
  (bind _playerlist (`self.playerlist`))
  (bind _playercrumbtodelete_i (break `/Game/Blueprints/Structs/BP_playerCrumb` (`local.playerCrumbToDelete`)))
  (bind _output_get (set `local.playerCrumbToDelete` (make `/Game/Blueprints/Structs/BP_playerCrumb` "")))
  (`SIOJLibrary.JsonObjectToStruct` (`SIOJLibrary.Conv_JsonValueToJsonObject` playerCrumb) _output_get)
  (set `local.playerToDelete` (`BlueprintMapLibrary.Map_Find` _playerlist _playercrumbtodelete_i))
  (`BlueprintMapLibrary.Map_Remove` _playerlist _playercrumbtodelete_i)
  (`self.K2_DestroyActor` (`local.playerToDelete`)))

(fn `setupProperties`
  (params (roomJSON :type "SIOJsonValue Object Reference"))
  (locals (roomCrumb :type "/Game/Blueprints/Structs/BP_roomCrumb Structure"))
  (bind (_roomcrumb_roomid _roomcrumb_name _roomcrumb_playercrumbs) (break `/Game/Blueprints/Structs/BP_roomCrumb` (`local.roomCrumb`)))
  (bind _output_get (set `local.roomCrumb` (make `/Game/Blueprints/Structs/BP_roomCrumb` "" "" (`|MakeArray` (struct) :!type "PlayerCrumb Structure"))))
  (bind _returnvalue (`SIOJLibrary.JsonObjectToStruct` (`SIOJLibrary.Conv_JsonValueToJsonObject` roomJSON) _output_get))
  (if _returnvalue
    (set `self.roomId` _roomcrumb_roomid)
    (set `self.name` _roomcrumb_name)
    (for _array_element _roomcrumb_playercrumbs
      (`self.addPlayer` _array_element))
    (`KismetSystemLibrary.PrintString` "Room setuup complete")))

(fn `UserConstructionScript`)