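; Point-and-click input actor that drives a world-space pointer and sends move requests on left click.
; BeginPlay spawns a BP_Pointer and enables player input; each Tick places it at the mouse's viewport position, normalized by viewport size and rescaled to fixed, negated world extents at Z zero.
; Left click passes the pointer's location to MoveTo on BP_CritalityInstance, the game instance.
; The mapping is pure arithmetic, with no trace or camera deprojection.
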(event `self.ReceiveBeginPlay`
  (bind _returnvalue (`|SpawnActorFromClass` "/Game/Blueprints/BP_Pointer.BP_Pointer_C" (`KismetMathLibrary.MakeTransform` (0.0 0.0 0.0)) "Undefined" "OverrideRootScale" self null))
  (set `self.Pointer` _returnvalue)
  (`self.EnableInput` (`GameplayStatics.GetPlayerController` 0)))

(event `self.ReceiveTick`
  (params (DeltaSeconds :type "Float (single-precision)"))
  (bind _returnvalue (`WidgetLayoutLibrary.GetMousePositionOnViewport`))
  (`self.K2_SetActorLocation` (`self.Pointer`) (`KismetMathLibrary.Conv_Vector2DToVector` (* (* (/ _returnvalue (`WidgetLayoutLibrary.GetViewportSize`)) (855.0 480.0)) -2.0)) false false))

(event `Key|LeftMouseButton`
  (params (Key :type "Key Structure"))
  (:`Pressed`
    (bind _asbp_critality_instance (cast `/Game/Blueprints/BP_CritalityInstance` (`GameplayStatics.GetGameInstance`)))
    (`/Game/Blueprints/BP_CritalityInstance.MoveTo` _asbp_critality_instance (`self.K2_GetActorLocation` (`self.Pointer`)))))

(fn `UserConstructionScript`)