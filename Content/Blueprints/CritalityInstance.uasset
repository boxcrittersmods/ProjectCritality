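; Game instance for Critality, a multiplayer client that opens the Menu level, manages menu and loading widgets, and owns the server connection.
; ConnectToServer creates a Socket.IO component, opening GameWorld on success or calling an empty error-display stub on failure.
; Login, movement, chat and emote events emit to the server, converting positions to Box Critters coordinates.
; Login sends a hardcoded sample player ID, and the connection Ticket is unused.
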(event `ShowMainMenu_VR`
  (params (UI :type "WidgetComponent Object Reference"))
  ;[1 1 1] Show VR Menu
  (`/Engine/EditorBlueprintResources/StandardMacros.IsValid` (`self.MainMenu_WB`)
    (:`Is Not Valid`
      (set `self.MainMenu_WB` (`WidgetComponent.GetUserWidgetObject` UI)))))

(event `self.ReceiveInit`
  ;[1 1 1] Start Game
  (`GameplayStatics.OpenLevel` "Menu"))

(event `ShowMainMenu`
  (bind _returnvalue (`GameplayStatics.GetPlayerController` 0))
  ;[1 1 1] Show Main Menu
  (`/Engine/EditorBlueprintResources/StandardMacros.IsValid` (`self.MainMenu_WB`)
    (:`Is Valid`
      _)
    (:`Is Not Valid`
      (bind _returnvalue_2 (`|CreateWidget` "/Game/Blueprints/Menu/BP_MainMenu.BP_MainMenu_C" _returnvalue))
      (bind _output_get (set `self.MainMenu_WB` _returnvalue_2))))
  (`UserWidget.AddToViewport` _output_get 0)
  (set `PlayerController.bShowMouseCursor` true _returnvalue))

(event `ShowLoadingScreen`
  ;[1 1 1] Show Loading Screen
  (`/Engine/EditorBlueprintResources/StandardMacros.IsValid` (`self.loadingScreen_WB`)
    (:`Is Valid`
      _)
    (:`Is Not Valid`
      (bind _returnvalue (`|CreateWidget` "/Game/Blueprints/Menu/BP_LoadingScreen.BP_LoadingScreen_C" (`GameplayStatics.GetPlayerController` 0)))
      (bind _output_get (set `self.loadingScreen_WB` _returnvalue))))
  (`UserWidget.AddToViewport` _output_get 0))

(event `ConnectToServer`
  (params (serverURL :type String) (username :type String) (ticket :type String))
  (bind _socket (`self.socket`))
  ;[1 1 1] Connect to Server
  (bind _output_get (set `self.serverURL` serverURL))
  (set `self.username` username)
  (`self.ShowLoadingScreen`)
  (bind _returnvalue (`SocketIOFunctionLibrary.ConstructSocketIOComponent`))
  (bind _output_get_2 (set `self.socket` _returnvalue))
  (`SocketIOClientComponent.Connect` _output_get_2 _output_get null null)
  (add `SocketIOClientComponent.OnConnected` _socket (delegate `SIO_Connected`))
  (add `SocketIOClientComponent.OnFail` _socket (delegate `SIO_Fail`)))

(event `self.ReceiveShutdown`
  (bind _socket (`self.socket`))
  ;[1 1 1] Disconnect
  (`/Engine/EditorBlueprintResources/StandardMacros.IsValid` _socket
    (:`Is Valid`
      (`SocketIOClientComponent.Emit` _socket "disconnect" (`SIOJsonValue.ConstructJsonValueString` "client closed") "/"))))

(event `SIO_Connected`
  (params (SessionId :type String) (bIsReconnection :type Boolean))
  ;[1 1 1] Connect to Server
  (`GameplayStatics.OpenLevel` "GameWorld"))

(event `SIO_Fail`
  ;[1 1 1] Connect to Server
  (`self.DisplayErrorMessage` "Failed to connect to server"))

(event `Login`
  ;[1 1 1] Login
  (bind _returnvalue (`SIOJsonObject.ConstructJsonObject`))
  (bind _output_get (set `self.id` "critalitySampleId"))
  (`SIOJsonObject.SetStringField` _returnvalue "playerId" _output_get)
  (`SIOJsonObject.SetStringField` _returnvalue "nickname" (`self.username`))
  (`SocketIOClientComponent.Emit` (`self.socket`) "login" (`SIOJsonValue.ConstructJsonValueObject` _returnvalue) "/"))

(event `MoveTo`
  (params (worldPos :type "Vector Structure"))
  ;[1 1 1] MoveTo
  (bind _returnvalue (`PosCoversion.UnrealToBoxCritters` worldPos))
  (`SocketIOClientComponent.Emit` (`self.socket`) "moveTo" (`SIOJsonValue.ConstructJsonValueArray` (`|MakeArray` (`SIOJsonValue.ConstructJsonValueNumber` (`KismetMathLibrary.BreakVector2D` _returnvalue)) (`SIOJsonValue.ConstructJsonValueNumber` (`.Y` (`KismetMathLibrary.BreakVector2D` _returnvalue))))) "/"))

(event `Message`
  (params (Message :type String))
  ;[1 1 1] Message
  (`SocketIOClientComponent.Emit` (`self.socket`) "message" (`SIOJsonValue.ConstructJsonValueString` Message) "/"))

(event `Emote`
  (params (message :type String))
  ;[1 1 1] Emote
  (`SocketIOClientComponent.Emit` (`self.socket`) "emote" (`SIOJsonValue.ConstructJsonValueString` message) "/"))